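; BoxAmmo is a projectile actor that flies toward the player and kills them on contact.
; On BeginPlay it captures the first ThirdPersonCharacter's mesh location once, so it does not home.
; The ShootTowardsPlayer timeline lerps it from InitialLocation to that point without sweep, destroying it when finished.
; Box overlap with a ThirdPersonCharacter destroys the projectile and calls KillPlayer.
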(event `self.ReceiveBeginPlay`
  (bind _outactors (`GameplayStatics.GetAllActorsOfClass` "/Game/ThirdPersonBP/Blueprints/ThirdPersonCharacter.ThirdPersonCharacter_C"))
  (bind _output (`|GetArrayItem` _outactors))
  (`/Engine/EditorBlueprintResources/StandardMacros.IsValid` _output
    (:`Is Valid`
      (set `self.PlayerLocation` (`SceneComponent.K2_GetComponentLocation` (`Character.Mesh` _output)))
      (bind (_direction _newtrack_0) (`Timeline|ShootTowardsPlayer` :!via `PlayFromStart`)
        (:`Update`
          (`self.K2_SetActorLocation` (`KismetMathLibrary.VLerp` (`self.InitialLocation`) (`self.PlayerLocation`) _newtrack_0)))
        (:`Finished`
          (`self.K2_DestroyActor`))))))

(event `self.Box.OnComponentBeginOverlap`
  (params (OverlappedComponent :type "PrimitiveComponent Object Reference") (OtherActor :type "Actor Object Reference") (OtherComp :type "PrimitiveComponent Object Reference") (OtherBodyIndex :type Integer) (bFromSweep :type Boolean) (SweepResult :type "HitResult Structure (by ref)"))
  (if (not (== OtherActor self))
    (bind _asthird_person_character (cast `/Game/ThirdPersonBP/Blueprints/ThirdPersonCharacter` OtherActor))
    (`self.K2_DestroyActor`)
    (`/Game/ThirdPersonBP/Blueprints/ThirdPersonCharacter.KillPlayer` _asthird_person_character)))

(fn `UserConstructionScript`)