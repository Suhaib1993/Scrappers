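; BodyAmmo is a projectile actor that travels a two-leg path and kills the player on contact.
; On BeginPlay it caches the world locations of PointA and PointB, then chains two timelines that lerp it from InitialLocation to PointA, then on to PointB.
; It destroys itself when the path ends.
; An overlap of Sphere1 with a ThirdPersonCharacter destroys it early and calls KillPlayer on that character.
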(event `self.ReceiveBeginPlay`
  (set `self.Point A` (`SceneComponent.K2_GetComponentLocation` (`self.PointA`)))
  (set `self.Point B` (`SceneComponent.K2_GetComponentLocation` (`self.PointB`)))
  (bind (_direction _delta) (`Timeline|Point1` :!via `PlayFromStart`)
    (:`Update`
      (`self.K2_SetActorLocation` (`KismetMathLibrary.VLerp` (`self.InitialLocation`) (`self.Point A`) _delta)))
    (:`Finished`
      (bind (_direction_2 _delta_2) (`Timeline|Point_2` :!via `PlayFromStart`)
        (:`Update`
          (`self.K2_SetActorLocation` (`KismetMathLibrary.VLerp` (`self.Point A`) (`self.Point B`) _delta_2)))
        (:`Finished`
          (`self.K2_DestroyActor`))))))

(event `self.Sphere1.OnComponentBeginOverlap`
  (params (OverlappedComponent :type "PrimitiveComponent Object Reference") (OtherActor :type "Actor Object Reference") (OtherComp :type "PrimitiveComponent Object Reference") (OtherBodyIndex :type Integer) (bFromSweep :type Boolean) (SweepResult :type "HitResult Structure (by ref)"))
  (bind _asthird_person_character (cast `/Game/ThirdPersonBP/Blueprints/ThirdPersonCharacter` OtherActor))
  (`self.K2_DestroyActor`)
  (`/Game/ThirdPersonBP/Blueprints/ThirdPersonCharacter.KillPlayer` _asthird_person_character))

(fn `UserConstructionScript`)