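; Enemy robot that attacks the player with randomly chained Level Sequence animations, spawned projectiles and a particle cannon kill box.
; BeginPlay creates the sequence players and binds their finish to replay a random one, leaving out the cannon when Life is zero.
; While IsActive, attack events spawn arm and body-gun ammo or toggle the kill box.
; An active kill box calls ParticleCanonKill on an overlapping ThirdPersonCharacter.
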(event `self.ReceiveBeginPlay`
  (`|ExecutionSequence`
    (:`then_0`
      (`self.RunAnimation`)
      (bind (_outactor _returnvalue) (`LevelSequencePlayer.CreateLevelSequencePlayer` "/Game/Cinematics/ArmAttack_Left.ArmAttack_Left"))
      (set `self.LeftArmAttack` _returnvalue)
      (bind (_outactor_2 _returnvalue_2) (`LevelSequencePlayer.CreateLevelSequencePlayer` "/Game/Cinematics/ArmAttack_Right.ArmAttack_Right"))
      (set `self.RightArmAttack` _returnvalue_2)
      (bind (_outactor_3 _returnvalue_3) (`LevelSequencePlayer.CreateLevelSequencePlayer` "/Game/Cinematics/Arms_Movement_1.Arms_Movement_1"))
      (set `self.ArmsWiggle1` _returnvalue_3)
      (bind (_outactor_4 _returnvalue_4) (`LevelSequencePlayer.CreateLevelSequencePlayer` "/Game/Cinematics/Arms_Movement_2.Arms_Movement_2"))
      (set `self.ArmsWiggle2` _returnvalue_4)
      (bind (_outactor_5 _returnvalue_5) (`LevelSequencePlayer.CreateLevelSequencePlayer` "/Game/Cinematics/BodyGuns.BodyGuns"))
      (set `self.BodyGun` _returnvalue_5)
      (bind (_outactor_6 _returnvalue_6) (`LevelSequencePlayer.CreateLevelSequencePlayer` "/Game/Cinematics/DualArm_Attack.DualArm_Attack"))
      (set `self.DualArmAttack` _returnvalue_6)
      (bind (_outactor_7 _returnvalue_7) (`LevelSequencePlayer.CreateLevelSequencePlayer` "/Game/Cinematics/ParticleCanon.ParticleCanon"))
      (set `self.ParticleCannon` _returnvalue_7))
    (:`then_1`
      (bind _output_get (set `self.AllSequences` (`|MakeArray` (`self.LeftArmAttack`) (`self.RightArmAttack`) (`self.ArmsWiggle1`) (`self.BodyGun`) (`self.DualArmAttack`) (`self.ArmsWiggle2`) (`self.ParticleCannon`))))
      (add `MovieSceneSequencePlayer.OnFinished` _output_get (delegate `PostAnimation`))
      (`self.RunAnimation`))))

(event `PostAnimation`
  (`KismetSystemLibrary.PrintString` "Hello")
  (`self.RunAnimation`))

(event `RunAnimation`
  (bind _output (`|GetArrayItem` (`self.AllSequences`) (`KismetMathLibrary.RandomIntegerInRange` 0 5)))
  (bind _output_2 (`|GetArrayItem` (`self.AllSequences`) (`KismetMathLibrary.RandomIntegerInRange` 0 6)))
  (if (== (`self.Life`) 0)
    (`/Engine/EditorBlueprintResources/StandardMacros.IsValid` _output
      (:`Is Valid`
        (`MovieSceneSequencePlayer.Play` _output)))
    (else
      (`/Engine/EditorBlueprintResources/StandardMacros.IsValid` _output_2
        (:`Is Valid`
          (`MovieSceneSequencePlayer.Play` _output_2))))))

(event `LeftAttack`
  (bind _returnvalue (`SceneComponent.K2_GetComponentToWorld` (`self.BoxAmmoLeft`)))
  (if (`self.IsActive`)
    (`|SpawnActorFromClass` "/Game/Blueprints/BoxAmmo.BoxAmmo_C" _returnvalue "Undefined" "OverrideRootScale" null (.location _returnvalue) null)))

(event `RightAttack`
  (bind _returnvalue (`SceneComponent.K2_GetComponentToWorld` (`self.BoxAmmoRight`)))
  (if (`self.IsActive`)
    (`|SpawnActorFromClass` "/Game/Blueprints/BoxAmmo.BoxAmmo_C" _returnvalue "Undefined" "OverrideRootScale" null (.location _returnvalue) null)))

(event `LeftAndRight`
  (`self.LeftAttack`)
  (`self.RightAttack`))

(event `BodyGunsAttack`
  (bind _returnvalue (`SceneComponent.K2_GetComponentLocation` (`self.Gun5Arrow`)))
  (bind _returnvalue_2 (`SceneComponent.K2_GetComponentLocation` (`self.Gun4Arrow`)))
  (bind _returnvalue_3 (`SceneComponent.K2_GetComponentLocation` (`self.Gun3Arrow`)))
  (bind _returnvalue_4 (`SceneComponent.K2_GetComponentLocation` (`self.Gun2Arrow`)))
  (bind _returnvalue_5 (`SceneComponent.K2_GetComponentLocation` (`self.Gun1Arrow`)))
  (bind _returnvalue_6 (`SceneComponent.K2_GetComponentLocation` (`self.GunArrow`)))
  (if (`self.IsActive`)
    (`|SpawnActorFromClass` "/Game/Blueprints/BodyAmmo.BodyAmmo_C" (`KismetMathLibrary.MakeTransform` _returnvalue_2 (struct :`Yaw` 180.0)) "Undefined" "OverrideRootScale" null _returnvalue_2 null)
    (`|SpawnActorFromClass` "/Game/Blueprints/BodyAmmo.BodyAmmo_C" (`KismetMathLibrary.MakeTransform` _returnvalue_3 (struct :`Yaw` 180.0)) "Undefined" "OverrideRootScale" null _returnvalue_3 null)
    (`|SpawnActorFromClass` "/Game/Blueprints/BodyAmmo.BodyAmmo_C" (`KismetMathLibrary.MakeTransform` _returnvalue_4 (struct :`Yaw` 180.0)) "Undefined" "OverrideRootScale" null _returnvalue_4 null)
    (`|SpawnActorFromClass` "/Game/Blueprints/BodyAmmo.BodyAmmo_C" (`KismetMathLibrary.MakeTransform` _returnvalue_5 (struct :`Yaw` 180.0)) "Undefined" "OverrideRootScale" null _returnvalue_5 null)
    (`|SpawnActorFromClass` "/Game/Blueprints/BodyAmmo.BodyAmmo_C" (`KismetMathLibrary.MakeTransform` _returnvalue_6 (struct :`Yaw` 180.0)) "Undefined" "OverrideRootScale" null _returnvalue_6 null)
    (`|SpawnActorFromClass` "/Game/Blueprints/BodyAmmo.BodyAmmo_C" (`KismetMathLibrary.MakeTransform` _returnvalue (struct :`Yaw` 180.0)) "Undefined" "OverrideRootScale" null _returnvalue null)))

(event `ParticleCanonActivate`
  (if (`self.IsActive`)
    (set `self.KillBoxActive?` true)))

(event `ParticleCanonDeactivate`
  (if (`self.IsActive`)
    (set `self.KillBoxActive?` false)))

(event `self.KillBox_Canon.OnComponentBeginOverlap`
  (params (OverlappedComponent :type "PrimitiveComponent Object Reference") (OtherActor :type "Actor Object Reference") (OtherComp :type "PrimitiveComponent Object Reference") (OtherBodyIndex :type Integer) (bFromSweep :type Boolean) (SweepResult :type "HitResult Structure (by ref)"))
  (if (`self.KillBoxActive?`)
    (bind _asthird_person_character (cast `/Game/ThirdPersonBP/Blueprints/ThirdPersonCharacter` OtherActor))
    (`/Game/ThirdPersonBP/Blueprints/ThirdPersonCharacter.ParticleCanonKill` _asthird_person_character)))

(fn `UserConstructionScript`)